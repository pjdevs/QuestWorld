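; BP_HackingTerminal is an interactable terminal that is hacked through a timed interaction of three seconds.
; Interaction input starts the phase, and ending that input early resets the timer and returns it to Ready.
; State feedback shows the progress widget and enables timing while Busy, then hides it otherwise.
; Tick feeds progress to the widget and completes the interaction as Interacted, which activates a Niagara effect.
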(event `self.OnStartInteractionInput`
  (params (InteractionInstigator :type "Actor Object Reference"))
  (set `self.HackingTime` 0.0)
  (`self.StartInteractionPhase` InteractionInstigator))

(event `self.OnEndInteractionInput`
  (params (InteractionInstigator :type "Actor Object Reference"))
  (set `self.HackingTime` 0.0)
  (`self.EndInteractionPhase` "Ready"))

(event `self.ReceiveTick`
  (params (DeltaSeconds :type "Float (single-precision)"))
  (bind _hackingtime (`self.HackingTime`))
  (if (`self.bIsHacking`)
    (set `self.HackingTime` (+ _hackingtime DeltaSeconds))
    (bind _aswbp_progress_hacking (cast `/Game/QuestWorld/Game/Interactables/WBP_ProgressHacking` (`WidgetComponent.GetUserWidgetObject` (`self.WidgetProgressHacking`))))
    (`/Game/QuestWorld/Game/Interactables/WBP_ProgressHacking.SetProgress` _aswbp_progress_hacking (/ _hackingtime 3.0))
    (if (>= (`self.HackingTime`) 3.0)
      (`self.EndInteractionPhase` "Interacted"))))

(event `self.DoFeedback`
  (params (NewState :type "IPInteractiveState Structure (by ref)"))
  (switch `EIPInteractiveState` NewState_State
    (:`Ready`
      (set `self.HackingTime` 0.0)
      (`SceneComponent.SetVisibility` (`self.WidgetProgressHacking`) false false)
      (set `self.bIsHacking` false))
    (:`Busy`
      (`SceneComponent.SetVisibility` (`self.WidgetProgressHacking`) true false)
      (set `self.bIsHacking` true))
    (:`Interacted`
      (set `self.HackingTime` 0.0)
      (`SceneComponent.SetVisibility` (`self.WidgetProgressHacking`) false false)
      (`ActorComponent.Activate` (`self.Niagara`) true)
      (set `self.bIsHacking` false))))

(fn `UserConstructionScript`)