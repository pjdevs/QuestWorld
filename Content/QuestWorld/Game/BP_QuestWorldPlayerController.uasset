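; Player controller for the quest world that owns the HUD and quest journal and reports player actions to the quest system.
; On BeginPlay it subscribes to the notification subsystem and creates the HUD, undoing both when destroyed.
; The journal input toggles a widget built from the active quests.
; The jump input calls StartQuest, then submits a "Jump" action quest event with itself as instigator.
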(event `self.ReceiveBeginPlay`
  (`NotificationSubsystem.Subscribe` (subsystem `NotificationSubsystem`) self)
  (`self.CreateHUD`))

(event `self.ReceiveDestroyed`
  (`NotificationSubsystem.Unsubscribe` (subsystem `NotificationSubsystem`) self)
  (`self.DestroyHUD`))

(event `EnhancedInput|/Game/QuestWorld/Input/Actions/IA_Journal`
  (params (ActionValue :type Boolean) (ElapsedSeconds :type "Float (double-precision)") (TriggeredSeconds :type "Float (double-precision)") (InputAction :type "InputAction Object Reference" :default "/Game/QuestWorld/Input/Actions/IA_Journal.IA_Journal"))
  (:`Started`
    (if (`self.IsQuestJournalOpened`)
      (`self.DestroyQuestJournal`)
      (else
        (`self.CreateQuestJournal`)))))

(event `EnhancedInput|/Game/QuestWorld/Input/Actions/IA_Jump`
  (params (ActionValue :type Boolean) (ElapsedSeconds :type "Float (double-precision)") (TriggeredSeconds :type "Float (double-precision)") (InputAction :type "InputAction Object Reference" :default "/Game/QuestWorld/Input/Actions/IA_Jump.IA_Jump"))
  (:`Triggered`
    (`QuestStatics.StartQuest` "Quest:DA_Quest_Jump")
    (bind _returnvalue (`|GenericCreateObject` "/Script/QuestSystem.ActionQuestEvent" "Jump" self))
    (`QuestStatics.SubmitQuestEvent` _returnvalue)))

(fn `CreateHUD`
  (bind _returnvalue (`|CreateWidget` "/Game/QuestWorld/UI/Widgets/WBP_HUD.WBP_HUD_C" self))
  (bind _output_get (set `self.HUD` _returnvalue))
  (`UserWidget.AddToViewport` _returnvalue 0)
  (`UserWidget.AddToViewport` _output_get 0))

(fn `CreateQuestJournal`
  (bind _returnvalue (`|CreateWidget` "/Game/QuestWorld/UI/Widgets/Quest/WBP_QuestJournal.WBP_QuestJournal_C" self (`QuestStatics.GetActiveQuests`)))
  (bind _output_get (set `self.QuestJournal` _returnvalue))
  (`UserWidget.AddToViewport` _output_get 0))

(fn `DestroyHUD`
  (bind _hud (`self.HUD`)
    (:`then`
      (`Widget.RemoveFromParent` _hud)
      (set `self.HUD` null))
    (:`else`)))

(fn `DestroyQuestJournal`
  (bind _questjournal (`self.QuestJournal`)
    (:`then`
      (`Widget.RemoveFromParent` _questjournal)
      (set `self.QuestJournal` null))
    (:`else`)))

(fn `IsQuestJournalOpened`
  (returns (IsOpened :type Boolean))
  (return (`KismetSystemLibrary.IsValid` (`self.QuestJournal`))))

(fn `UserConstructionScript`)